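; BP_Sword is a player sword Blueprint that plays a sound when the blade is swung fast.
; Each Tick it estimates tip speed from how far its Scene component moved since the last frame, then stores the new location.
; Above a speed threshold, it plays Sword_Cue at the tip with speed-scaled, clamped volume, using a DoOnce with delayed reset as a one-second cooldown.
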(event `self.ReceiveTick`
  (params (DeltaSeconds :type "Float (single-precision)"))
  (bind _returnvalue (`SceneComponent.K2_GetComponentLocation` (`self.Scene`)))
  (bind _returnvalue_2 (/ (`KismetMathLibrary.Vector_Distance` _returnvalue (`self.lastTipLocation`)) DeltaSeconds))
  (`|ExecutionSequence`
    (:`then_0`
      (if (> _returnvalue_2 800.0)
        (`self.playSound` (/ _returnvalue_2 2000.0))))
    (:`then_1`
      (set `self.lastTipLocation` _returnvalue))))

(event `playSound`
  (params (volume :type "Float (double-precision)"))
  (`/Engine/EditorBlueprintResources/StandardMacros.DoOnce` false :!label _label
    (:`Completed`
      (`|ExecutionSequence`
        (:`then_0`
          (`GameplayStatics.PlaySoundAtLocation` "/Game/Audio/SFX/sword_Cue.sword_Cue" (`self.lastTipLocation`) (struct) (`KismetMathLibrary.FClamp` volume) 1.0 0.0 null null null null))
        (:`then_1`
          (`KismetSystemLibrary.Delay` 1.0)
          (goto _label :!via `Reset`))))))

(fn `UserConstructionScript`)