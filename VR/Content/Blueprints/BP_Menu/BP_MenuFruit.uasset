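; BP_MenuFruit is a floating, sliceable fruit for the menu, with a text label.
; It starts at a random rotation with projectile velocity and gravity zeroed, then spins every tick.
; A one-shot onHit event hides the fruit and label, spawns an effect, plays hit and random water sounds, then self-destroys after a delay.
; It also spawns BP_Chunks, passing materials cached at construction and a scale derived from the collision sphere radius.
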(event `self.ReceiveBeginPlay`
  (bind _projectilemovement (`self.ProjectileMovement`))
  (`SceneComponent.K2_SetWorldRotation` (`self.Container`) (`KismetMathLibrary.MakeRotator` (`KismetMathLibrary.RandomFloatInRange` -180.0 180.0) (`KismetMathLibrary.RandomFloatInRange` -180.0 180.0) (`KismetMathLibrary.RandomFloatInRange` -180.0 180.0)) false false)
  ;[1 1 1] For Menu Fruit Physics Settings
  (set `ProjectileMovementComponent.InitialSpeed` 0.0 _projectilemovement)
  (`ProjectileMovementComponent.SetVelocityInLocalSpace` _projectilemovement (`KismetMathLibrary.MakeVector` 0.0))
  (set `ProjectileMovementComponent.ProjectileGravityScale` 0.0 _projectilemovement))

(event `self.ReceiveTick`
  (params (DeltaSeconds :type "Float (single-precision)"))
  (`SceneComponent.K2_AddWorldRotation` (`self.Container`) (struct :`Roll` 5.0) false false))

(event `onHit`
  (bind _hitsoundwater (`self.HitSoundWater`))
  ;[1 1 1] On Hit
  (`/Engine/EditorBlueprintResources/StandardMacros.DoOnce` false
    (:`Completed`
      (`|ExecutionSequence`
        (:`then_0`
          (`SceneComponent.SetVisibility` (`self.FruitMesh`) false false)
          (`SceneComponent.SetVisibility` (`self.CollisionMesh`) false false)
          (`SceneComponent.SetVisibility` (`self.TextRender`) false false)
          (`|ExecutionSequence`
            (:`then_0`
              (`NiagaraFunctionLibrary.SpawnSystemAtLocation` (`self.Effect`) (`self.K2_GetActorLocation`)))
            (:`then_1`
              (`|SpawnActorFromClass` "/Game/Blueprints/BP_Fruit/BP_Chunks.BP_Chunks_C" (`self.GetTransform`) "Undefined" "MultiplyWithRoot" null (`self.MainMaterial`) (`self.ChunkMaterial`) (/ (`SphereComponent.SphereRadius` (`self.CollisionMesh`)) 21.0) null))
            (:`then_3`
              (`ActorComponent.K2_DestroyComponent` (`self.CollisionMesh`)))))
        (:`then_1`
          (`KismetSystemLibrary.Delay` 1.0)
          (`self.K2_DestroyActor`))
        (:`then_2`
          (`AudioComponent.Play` (`self.HitSound`) 0.0)
          (`AudioComponent.SetSound` _hitsoundwater (select `int` (`KismetMathLibrary.RandomIntegerInRange` 0 2) :`0` "/Game/Audio/FruitSound/blade_water1_Cue.blade_water1_Cue" :`1` "/Game/Audio/FruitSound/blade_water2_Cue.blade_water2_Cue" :`2` "/Game/Audio/FruitSound/blade_water3_Cue.blade_water3_Cue" :!type "SoundCue Object Reference"))
          (`AudioComponent.Play` _hitsoundwater 0.0))))))

(fn `UserConstructionScript`
  (bind _fruitmesh (`self.FruitMesh`))
  (set `self.MainMaterial` (`PrimitiveComponent.GetMaterial` _fruitmesh 0))
  (set `self.ChunkMaterial` (`PrimitiveComponent.GetMaterial` _fruitmesh 1)))