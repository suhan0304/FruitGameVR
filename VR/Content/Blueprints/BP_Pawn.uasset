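; VR player pawn with camera-relative movement, snap turning that keeps the camera in place, and a pause toggle.
; BeginPlay adds the input mapping, calibrates VRRoot to the desired camera height, and spawns two BP_Hand actors that handle grab and release.
; Tick rebuilds a right-hand spline mesh toward hovered widgets, but immediately hides it.
; Left-hand pointer and pause-menu widget logic are unwired, so pausing only freezes the game.
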(event `self.ReceiveBeginPlay`
  (bind (_returnvalue_x _returnvalue_y _returnvalue_z) (`KismetMathLibrary.BreakVector` (`SceneComponent.K2_GetComponentLocation` (`self.Camera`))))
  (`|ExecutionSequence`
    (:`then_0`
      (`EnhancedInputSubsystemInterface.AddMappingContext` (pcsubsystem `EnhancedInputLocalPlayerSubsystem` (`GameplayStatics.GetPlayerController` 0)) "/Game/Blueprints/Input/IMC_VR_Default.IMC_VR_Default" 0 (struct)))
    (:`then_1`
      (`/Engine/EditorBlueprintResources/StandardMacros.DoOnce` false
        (:`Completed`
          (`HeadMountedDisplayFunctionLibrary.SetTrackingOrigin` "Floor")
          (`KismetSystemLibrary.Delay` 1.0)
          (`SceneComponent.K2_AddRelativeLocation` (`self.VRRoot`) (`KismetMathLibrary.MakeVector` 0.0 0.0 (- (`self.DesiredCameraHeight`) _returnvalue_z)) false false))))
    (:`then_2`
      (bind _returnvalue (`|SpawnActorFromClass` "/Game/Blueprints/BP_Hand.BP_Hand_C" (`KismetMathLibrary.MakeTransform` (0.0 0.0 0.0)) "AlwaysSpawn" "MultiplyWithRoot" self true null))
      (bind _output_get (set `self.LeftHand` _returnvalue))
      (`self.K2_AttachToComponent` _output_get (`self.VRRoot`) "None" "SnapToTarget" "SnapToTarget" "KeepWorld" true))
    (:`then_3`
      (bind _returnvalue_2 (`|SpawnActorFromClass` "/Game/Blueprints/BP_Hand.BP_Hand_C" (`KismetMathLibrary.MakeTransform` (0.0 0.0 0.0)) "AlwaysSpawn" "MultiplyWithRoot" self false null))
      (bind _output_get_2 (set `self.RightHand` _returnvalue_2))
      (`self.K2_AttachToComponent` _output_get_2 (`self.VRRoot`) "None" "SnapToTarget" "SnapToTarget" "KeepWorld" true))))

(event `EnhancedInput|/Game/Blueprints/Input/Actions/IA_VR_Move`
  (params (ActionValue :type "Float (double-precision)") (ElapsedSeconds :type "Float (double-precision)") (TriggeredSeconds :type "Float (double-precision)") (InputAction :type "InputAction Object Reference" :default "/Game/Blueprints/Input/Actions/IA_VR_Move.IA_VR_Move"))
  (bind (_returnvalue_x _returnvalue_y) (`KismetMathLibrary.BreakVector` (`SceneComponent.GetForwardVector` (`self.Camera`))))
  (:`Triggered`
    (`self.AddMovementInput` (`KismetMathLibrary.MakeVector` _returnvalue_x _returnvalue_y) ActionValue)))

(event `EnhancedInput|/Game/Blueprints/Input/Actions/IA_VR_MoveSide`
  (params (ActionValue :type "Float (double-precision)") (ElapsedSeconds :type "Float (double-precision)") (TriggeredSeconds :type "Float (double-precision)") (InputAction :type "InputAction Object Reference" :default "/Game/Blueprints/Input/Actions/IA_VR_MoveSide.IA_VR_MoveSide"))
  (bind (_returnvalue_x _returnvalue_y) (`KismetMathLibrary.BreakVector` (`SceneComponent.GetRightVector` (`self.Camera`))))
  (:`Triggered`
    (`self.AddMovementInput` (`KismetMathLibrary.MakeVector` _returnvalue_x _returnvalue_y) ActionValue)))

(event `EnhancedInput|/Game/Blueprints/Input/Actions/IA_VR_Turn`
  (params (ActionValue :type "Float (double-precision)") (ElapsedSeconds :type "Float (double-precision)") (TriggeredSeconds :type "Float (double-precision)") (InputAction :type "InputAction Object Reference" :default "/Game/Blueprints/Input/Actions/IA_VR_Turn.IA_VR_Turn"))
  (:`Started`
    (`self.SnapTurn` (> ActionValue 0.0))))

(event `EnhancedInput|/Game/Blueprints/Input/Actions/IA_VR_Grab_Left`
  (params (ActionValue :type "Float (double-precision)") (ElapsedSeconds :type "Float (double-precision)") (TriggeredSeconds :type "Float (double-precision)") (InputAction :type "InputAction Object Reference" :default "/Game/Blueprints/Input/Actions/IA_VR_Grab_Left.IA_VR_Grab_Left"))
  (bind _lefthand (`self.LeftHand`))
  (:`Started`
    (`/Game/Blueprints/BP_Hand.HandleGrab` _lefthand))
  (:`Completed`
    (`/Game/Blueprints/BP_Hand.HandleRelease` _lefthand)))

(event `EnhancedInput|/Game/Blueprints/Input/Actions/IA_VR_Grab_Right`
  (params (ActionValue :type "Float (double-precision)") (ElapsedSeconds :type "Float (double-precision)") (TriggeredSeconds :type "Float (double-precision)") (InputAction :type "InputAction Object Reference" :default "/Game/Blueprints/Input/Actions/IA_VR_Grab_Right.IA_VR_Grab_Right"))
  (bind _righthand (`self.RightHand`))
  (:`Started`
    (`/Game/Blueprints/BP_Hand.HandleGrab` _righthand))
  (:`Completed`
    (`/Game/Blueprints/BP_Hand.HandleRelease` _righthand)))

(event `self.ReceiveTick`
  (params (DeltaSeconds :type "Float (single-precision)"))
  (`self.WidgetInteractionPointer` (`self.RightHand`)))

(event `EnhancedInput|/Game/Blueprints/Input/Actions/IA_Pause_Game`
  (params (ActionValue :type Boolean) (ElapsedSeconds :type "Float (double-precision)") (TriggeredSeconds :type "Float (double-precision)") (InputAction :type "InputAction Object Reference" :default "/Game/Blueprints/Input/Actions/IA_Pause_Game.IA_Pause_Game"))
  ;[1 1 1] pauseGame
  (:`Started`
    (if (not (`self.isPauseMenuOpened?`))
      (set `self.isPauseMenuOpened?` true)
      (`GameplayStatics.SetGamePaused` true)
      (else
        (set `self.isPauseMenuOpened?` false)
        (`GameplayStatics.SetGamePaused` false)))))

(fn `SnapTurn`
  (params (bRightTurn :type Boolean))
  (locals (LocalYawDelta :type "Float (double-precision)") (LocalPrevCameraLocation :type "Vector Structure"))
  (bind _snapturndegrees (`self.SnapTurnDegrees`))
  (set `local.LocalPrevCameraLocation` (`SceneComponent.K2_GetComponentLocation` (`self.Camera`)))
  (`self.K2_AddActorWorldRotation` (`KismetMathLibrary.MakeRotator` 0.0 0.0 (`KismetMathLibrary.SelectFloat` (`KismetMathLibrary.Abs` _snapturndegrees) _snapturndegrees (`local.bRightTurn`))) false true)
  (`self.K2_AddActorWorldOffset` (- (`local.LocalPrevCameraLocation`) (`SceneComponent.K2_GetComponentLocation` (`self.Camera`))) false true))

(fn `UserConstructionScript`)

(fn `WidgetInteractionPointer`
  (params (RightHand :type "/Game/Blueprints/BP_Hand Object Reference"))
  (locals (NewLocalVar :type "SplineMeshComponent Object Reference"))
  (bind _widgetinteraction (`/Game/Blueprints/BP_Hand.WidgetInteraction` RightHand))
  (bind _returnvalue (`SceneComponent.K2_GetComponentLocation` _widgetinteraction))
  (bind (_returnvalue_bblockinghit _returnvalue_binitialoverlap _returnvalue_time _returnvalue_distance _returnvalue_location) (`GameplayStatics.BreakHitResult` (`WidgetInteractionComponent.GetLastHitResult` _widgetinteraction)))
  (bind _returnvalue_2 (`KismetMathLibrary.GetForwardVector` (`KismetMathLibrary.FindLookAtRotation` _returnvalue _returnvalue_location)))
  ;[1 1 1] Right Hand
  (bind _rightsplinemesh (`self.RightSplineMesh`)
    (:`then`
      (`ActorComponent.K2_DestroyComponent` _rightsplinemesh))
    (:`else`
      _))
  (if (`WidgetInteractionComponent.IsOverHitTestVisibleWidget` _widgetinteraction)
    (bind _returnvalue_3 (`AddComponent|NODE_AddSplineMeshComponent-1` :`bManualAttachment` true))
    (bind _output_get (set `self.RightSplineMesh` _returnvalue_3))
    (`SplineMeshComponent.SetStartAndEnd` _output_get _returnvalue _returnvalue_2 _returnvalue_location (* _returnvalue_2 (`KismetMathLibrary.Conv_DoubleToVector` -1.0)) true)
    (`SceneComponent.SetVisibility` _returnvalue_3 false false)))