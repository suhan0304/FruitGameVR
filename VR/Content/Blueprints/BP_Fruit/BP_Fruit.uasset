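; BP_Fruit is a projectile fruit actor that is launched in an upward arc and bursts into chunks when hit.
; On BeginPlay it randomizes rotation and aims velocity near BP_FruitManager's End point, or floats motionless in debug mode.
; A one-shot onHit hides the fruit, spawns an effect and size-scaled BP_Chunks using materials cached in construction, plays slice sounds, then destroys the actor after a delay.
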(event `self.ReceiveBeginPlay`
  (bind _projectilemovement (`self.ProjectileMovement`))
  (bind _projectilemovement_2 (`self.ProjectileMovement`))
  (`SceneComponent.K2_SetWorldRotation` (`self.Container`) (`KismetMathLibrary.MakeRotator` (`KismetMathLibrary.RandomFloatInRange` -180.0 180.0) (`KismetMathLibrary.RandomFloatInRange` -180.0 180.0) (`KismetMathLibrary.RandomFloatInRange` -180.0 180.0)) false false)
  (if (`self.ForDebug`)
    ;[1 1 1] For Test Fruit Physics Settings
    (set `ProjectileMovementComponent.InitialSpeed` 0.0 _projectilemovement_2)
    (`ProjectileMovementComponent.SetVelocityInLocalSpace` _projectilemovement_2 (`KismetMathLibrary.MakeVector` 0.0))
    (set `ProjectileMovementComponent.ProjectileGravityScale` 0.0 _projectilemovement_2)
    (else
      ;[1 1 1] For Play Fruit Physics Settings
      (bind _returnvalue (`GameplayStatics.GetActorOfClass` "/Game/Blueprints/BP_FruitManager.BP_FruitManager_C"))
      (set `MovementComponent.Velocity` (`KismetMathLibrary.MakeVector` (- (.x (`KismetMathLibrary.RandomPointInBoundingBox` (`SceneComponent.K2_GetComponentLocation` (`/Game/Blueprints/BP_FruitManager.End` _returnvalue)) (10.0 10.0 10.0))) (.x (`SceneComponent.K2_GetComponentLocation` (`self.CollisionMesh`)))) (- (.y (`KismetMathLibrary.RandomPointInBoundingBox` (`SceneComponent.K2_GetComponentLocation` (`/Game/Blueprints/BP_FruitManager.End` _returnvalue)) (10.0 10.0 10.0))) (.y (`SceneComponent.K2_GetComponentLocation` (`self.CollisionMesh`)))) 600.0) _projectilemovement)
      (set `ProjectileMovementComponent.ProjectileGravityScale` 1.0 _projectilemovement))))

(event `onHit`
  (bind _hitsoundwater (`self.HitSoundWater`))
  ;[1 1 1] On Hit
  (`/Engine/EditorBlueprintResources/StandardMacros.DoOnce` false
    (:`Completed`
      (`|ExecutionSequence`
        (:`then_0`
          (`SceneComponent.SetVisibility` (`self.FruitMesh`) false false)
          (`SceneComponent.SetVisibility` (`self.CollisionMesh`) false false)
          (`|ExecutionSequence`
            (:`then_0`
              (`NiagaraFunctionLibrary.SpawnSystemAtLocation` (`self.Effect`) (`self.K2_GetActorLocation`)))
            (:`then_1`
              (`|SpawnActorFromClass` "/Game/Blueprints/BP_Fruit/BP_Chunks.BP_Chunks_C" (`self.GetTransform`) "Undefined" "MultiplyWithRoot" null (`self.MainMaterial`) (`self.ChunkMaterial`) (/ (`SphereComponent.SphereRadius` (`self.CollisionMesh`)) 21.0) null))
            (:`then_3`
              (`ActorComponent.K2_DestroyComponent` (`self.CollisionMesh`)))))
        (:`then_1`
          (`KismetSystemLibrary.Delay` 1.0)
          (`self.K2_DestroyActor`))
        (:`then_2`
          (`AudioComponent.Play` (`self.HitSound`) 0.0)
          (`AudioComponent.SetSound` _hitsoundwater (select `int` (`KismetMathLibrary.RandomIntegerInRange` 0 2) :`0` "/Game/Audio/FruitSound/blade_water1_Cue.blade_water1_Cue" :`1` "/Game/Audio/FruitSound/blade_water2_Cue.blade_water2_Cue" :`2` "/Game/Audio/FruitSound/blade_water3_Cue.blade_water3_Cue" :!type "SoundCue Object Reference"))
          (`AudioComponent.Play` _hitsoundwater 0.0))))))

(fn `UserConstructionScript`
  (bind _fruitmesh (`self.FruitMesh`))
  (set `self.MainMaterial` (`PrimitiveComponent.GetMaterial` _fruitmesh 0))
  (set `self.ChunkMaterial` (`PrimitiveComponent.GetMaterial` _fruitmesh 1)))