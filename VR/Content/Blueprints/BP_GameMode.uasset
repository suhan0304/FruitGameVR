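; Game mode for a fruit game that tracks the total score and controls the start and end of rounds.
; Start events for the normal and "Sixty" modes reset the score, then tell the BP_FruitManager found in the level to start and hide the score display.
; Stopping, also triggered when health hits zero, passes the total to the manager to show and halts it.
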(event `StartSixtyGame`
  (set `self.totalScore` 0)
  (`|ExecutionSequence`
    (:`then_0`
      (bind _returnvalue (`GameplayStatics.GetActorOfClass` "/Game/Blueprints/BP_FruitManager.BP_FruitManager_C"))
      (`/Engine/EditorBlueprintResources/StandardMacros.IsValid` _returnvalue
        (:`Is Valid`
          (`/Game/Blueprints/BP_FruitManager.StartSixtyGame` _returnvalue))))
    (:`then_1`
      (bind _returnvalue_2 (`GameplayStatics.GetActorOfClass` "/Game/Blueprints/BP_FruitManager.BP_FruitManager_C"))
      (`/Game/Blueprints/BP_FruitManager.hideScore` _returnvalue_2))))

(event `self.ReceiveBeginPlay`)

(event `StartGame`
  (set `self.totalScore` 0)
  (`|ExecutionSequence`
    (:`then_0`
      (bind _returnvalue (`GameplayStatics.GetActorOfClass` "/Game/Blueprints/BP_FruitManager.BP_FruitManager_C"))
      (`/Engine/EditorBlueprintResources/StandardMacros.IsValid` _returnvalue
        (:`Is Valid`
          (`/Game/Blueprints/BP_FruitManager.StartGame` _returnvalue))))
    (:`then_1`
      (bind _returnvalue_2 (`GameplayStatics.GetActorOfClass` "/Game/Blueprints/BP_FruitManager.BP_FruitManager_C"))
      (`/Game/Blueprints/BP_FruitManager.hideScore` _returnvalue_2))))

(event `StopGame`
  (`|ExecutionSequence`
    (:`then_0`
      (bind _returnvalue (`GameplayStatics.GetActorOfClass` "/Game/Blueprints/BP_FruitManager.BP_FruitManager_C"))
      (`/Game/Blueprints/BP_FruitManager.showScore` _returnvalue (`self.totalScore`)))
    (:`then_1`
      (bind _returnvalue_2 (`GameplayStatics.GetActorOfClass` "/Game/Blueprints/BP_FruitManager.BP_FruitManager_C"))
      (`/Engine/EditorBlueprintResources/StandardMacros.IsValid` _returnvalue_2
        (:`Is Valid`
          (`/Game/Blueprints/BP_FruitManager.StopGame` _returnvalue_2))))))

(event `addScore`
  (params (Score :type Integer))
  (set `self.totalScore` (+ Score (`self.totalScore`))))

(event `onHealthZero`
  (`self.StopGame`))

(fn `UserConstructionScript`)