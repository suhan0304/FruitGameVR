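; BP_Itembox is an item box actor that displays a randomly chosen item: a pumpkin, fish or mushroom.
; On BeginPlay it rolls ItemNumber, selects the matching static mesh and applies it with its first material to FruitMesh.
; The mushroom variant is scaled down before the parent BeginPlay runs.
; The construction script only calls the parent, and this Blueprint adds no other logic.
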(event `self.ReceiveBeginPlay`
  (bind _output_get (set `self.ItemNumber` (`KismetMathLibrary.RandomIntegerInRange` 0 2)))
  (bind _output_get_2 (set `self.mesh` (select `int` _output_get :`0` "/Game/Meshes/SM_Pumkin1.SM_Pumkin1" :`1` "/Game/Meshes/SM_Fish1.SM_Fish1" :`2` "/Game/Meshes/SM_Mushroom_Var04.SM_Mushroom_Var04" :!type "StaticMesh Object Reference")))
  (`StaticMeshComponent.SetStaticMesh` (`self.FruitMesh`) _output_get_2)
  (`PrimitiveComponent.SetMaterial` (`self.FruitMesh`) 0 (`StaticMesh.GetMaterial` _output_get_2 0))
  (if (== (`self.mesh`) "/Game/Meshes/SM_Mushroom_Var04.SM_Mushroom_Var04")
    (`SceneComponent.SetWorldScale3D` (`self.FruitMesh`) (0.75 0.75 0.75)))
  (`parent.ReceiveBeginPlay`))

(fn `UserConstructionScript`
  (`parent.UserConstructionScript`))