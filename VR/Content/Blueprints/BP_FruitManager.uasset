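; Manager actor for a fruit-hitting game, running spawning, health, HUD and menu fruits for normal and 60-second modes.
; Self-rescheduling timers launch random objects from an arc facing a target point.
; Normal mode adds bombs and item boxes, with rising difficulty enlarging bursts and raising music pitch; timed mode is damage-free.
; Fruits reaching the miss box drain health, ending the game via GameMode; StopGame clears fruits and restores menu fruits.
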(event `removeAllMenu`
  ;[1 1 1] 모든 메뉴과일 파괴
  (bind _outactors (`GameplayStatics.GetAllActorsOfClass` "/Game/Blueprints/BP_Menu/BP_MenuFruit.BP_MenuFruit_C"))
  (for _array_element _outactors
    (`self.K2_DestroyActor` _array_element)))

(event `StopGame`
  ;[1 1 1] 게임 종료시
  (`|ExecutionSequence`
    (:`then_0`
      (`KismetSystemLibrary.K2_ClearAndInvalidateTimerHandle` (`self.nextDifficultyTimer`)))
    (:`then_1`
      (`KismetSystemLibrary.K2_ClearAndInvalidateTimerHandle` (`self.nextSpawnTimer`)))
    (:`then_2`
      (`self.removeAllFruits`))
    (:`then_3`
      (`|SpawnActorFromClass` "/Game/Blueprints/BP_Menu/BP_StartMenuFruit.BP_StartMenuFruit_C" (`KismetMathLibrary.MakeTransform` (-650.0 -40.0 25.0)) "Undefined" "MultiplyWithRoot" null "/Game/FruitAssetsMS/MS_Fruits/3D_Asset/14_Watermelon_tguocjppa/14_Watermelon_tguocjppa_8K_inst.14_Watermelon_tguocjppa_8K_inst" "/Game/FruitAssetsMS/MS_Fruits/3D_Asset/22_Red_Apple_tgzoahbpa/22_Red_Apple_tgzoahbpa_8K_inst.22_Red_Apple_tgzoahbpa_8K_inst" null)
      (`|SpawnActorFromClass` "/Game/Blueprints/BP_Menu/BP_ToMainMenuFruit.BP_ToMainMenuFruit_C" (`KismetMathLibrary.MakeTransform` (-650.0 40.0 25.0)) "Undefined" "MultiplyWithRoot" null null null null))
    (:`then_4`
      (`|SpawnActorFromClass` "/Game/Blueprints/BP_Menu/BP_SixtyStartMenuFruit.BP_SixtyStartMenuFruit_C" (`KismetMathLibrary.MakeTransform` (-620.0 -130.0 25.0)) "Undefined" "MultiplyWithRoot" null null null null))
    (:`then_5`
      (`self.ResetDifficulty`))
    (:`then_6`
      (`self.HideHUD`)
      (`self.stopTimer`))))

(event `self.ReceiveBeginPlay`
  ;[1 1 1] 레벨 첫 접근시
  (`KismetSystemLibrary.ExecuteConsoleCommand` "stat fps" null))

(event `removeAllFruits`
  ;[1 1 1] 모든 과일 파괴
  (bind _outactors (`GameplayStatics.GetAllActorsOfClass` "/Game/Blueprints/BP_Fruit/BP_Fruit.BP_Fruit_C"))
  (for _array_element _outactors
    (`self.K2_DestroyActor` _array_element)))

(event `showScore`
  (params (Score :type Integer))
  (bind _widgetgameresults (`self.WidgetGameResults`))
  ;[1 1 1] 점수 표시
  (`|ExecutionSequence`
    (:`then_0`
      (bind _aswgt_game_results (cast `/Game/Widget/WGT_GameResults` (`WidgetComponent.GetUserWidgetObject` _widgetgameresults)))
      (`/Game/Widget/WGT_GameResults.updateScoreValue` _aswgt_game_results Score))
    (:`then_1`
      (`SceneComponent.SetVisibility` _widgetgameresults true false))))

(event `StartSixtyGame`
  ;[1 1 1] 60초 게임 시작시
  (`|ExecutionSequence`
    (:`then_0`
      (set `self.DamagerPerFruit` 0.0))
    (:`then_1`
      (bind _output_get (set `self.Health` 100.0))
      (bind _ashud (cast `/Game/UI/HUD` (`WidgetComponent.GetUserWidgetObject` (`self.HUDWidget`))))
      (set `/Game/UI/HUD.HealthPercentage` _output_get _ashud))
    (:`then_2`
      (`self.ShowHUD`)
      (`self.startTimer`))
    (:`then_3`
      (`self.removeAllMenu`)
      (`KismetSystemLibrary.Delay` 3.0))
    (:`then_4`
      (`self.SpawnFruitSixty`)
      (`KismetSystemLibrary.Delay` 60.0)
      (`self.StopGame`)
      (bind _asbp_game_mode (cast `/Game/Blueprints/BP_GameMode` (`GameplayStatics.GetGameMode`)))
      (`/Game/Blueprints/BP_GameMode.StopGame` _asbp_game_mode))))

(event `hideScore`
  ;[1 1 1] 점수 숨기기
  (`SceneComponent.SetVisibility` (`self.WidgetGameResults`) false false))

(event `IncreaseDifficulty`
  (bind _music1_cue (`self.music1_Cue`))
  ;[1 1 1] 난이도 상승
  (`|ExecutionSequence`
    (:`then_0`
      (`|ExecutionSequence`
        (:`then_0`
          (`KismetSystemLibrary.PrintString` "Difficulty Increase!")
          (`AudioComponent.SetPitchMultiplier` _music1_cue (+ 0.1 (`AudioComponent.PitchMultiplier` _music1_cue))))
        (:`then_1`
          (set `self.Difficulty` (+ (`self.Difficulty`) 1.0)))))
    (:`then_1`
      (bind _returnvalue (`KismetSystemLibrary.K2_SetTimerDelegate` (delegate `IncreaseDifficulty`) (`self.DifficultyIncreaseInterval`)))
      (set `self.nextDifficultyTimer` _returnvalue))))

(event `StartGame`
  ;[1 1 1] 게임 시작시
  (`|ExecutionSequence`
    (:`then_0`
      (set `self.Difficulty` 0.0)
      (set `self.DamagerPerFruit` 10.0))
    (:`then_1`
      (bind _output_get (set `self.Health` 100.0))
      (bind _ashud (cast `/Game/UI/HUD` (`WidgetComponent.GetUserWidgetObject` (`self.HUDWidget`))))
      (set `/Game/UI/HUD.HealthPercentage` _output_get _ashud))
    (:`then_2`
      (`self.ShowHUD`)
      (`self.startTimer`))
    (:`then_3`
      (`KismetSystemLibrary.Delay` 3.0)
      (`|ExecutionSequence`
        (:`then_0`
          (`self.IncreaseDifficulty`))
        (:`then_1`
          (`self.Spawn Fruit`))))
    (:`then_4`
      (`self.removeAllMenu`))))

(event `ShowHUD`
  ;[1 1 1] HUD 표시
  (`SceneComponent.SetVisibility` (`self.HUDWidget`) true false))

(event `HideHUD`
  ;[1 1 1] HUD 숨기기
  (`SceneComponent.SetVisibility` (`self.HUDWidget`) false false))

(event `ResetDifficulty`
  ;[1 1 1] 난이도 초기화
  (set `self.Difficulty` 0.0)
  (`AudioComponent.SetPitchMultiplier` (`self.music1_Cue`) 1.0))

(event `self.Box.OnComponentBeginOverlap`
  (params (OverlappedComponent :type "PrimitiveComponent Object Reference") (OtherActor :type "Actor Object Reference") (OtherComp :type "PrimitiveComponent Object Reference") (OtherBodyIndex :type Integer) (bFromSweep :type Boolean) (SweepResult :type "HitResult Structure (by ref)"))
  (bind _returnvalue (`GameplayStatics.GetObjectClass` OtherActor))
  ;[1 1 1] 오브젝트 타격 실패 처리
  (if (or (== "/Game/Blueprints/BP_Items/BP_Bomb.BP_Bomb_C" _returnvalue) (== _returnvalue "/Game/Blueprints/BP_Items/BP_Itembox.BP_Itembox_C"))
    (`self.K2_DestroyActor` OtherActor)
    (else
      (bind _asbp_fruit (cast `/Game/Blueprints/BP_Fruit/BP_Fruit` OtherActor))
      (`self.fruitFailed` _asbp_fruit))))

(event `startTimer`
  ;[1 1 1] 타이머 시작
  (`|ExecutionSequence`
    (:`then_0`
      (`KismetSystemLibrary.PrintString` "Pawn called \"set Timer Started\""))
    (:`then_1`
      (bind _ashud (cast `/Game/UI/HUD` (`WidgetComponent.GetUserWidgetObject` (`self.HUDWidget`))))
      (`/Game/UI/HUD.setTimerStarted` _ashud))))

(event `fruitFailed`
  (params (Fruit :type "/Game/Blueprints/BP_Fruit/BP_Fruit Object Reference"))
  ;[1 1 1] 과일 타격 실패시
  (`|ExecutionSequence`
    (:`then_0`
      (cast `/Game/Blueprints/BP_GameMode` (`GameplayStatics.GetGameMode`))
      (`|ExecutionSequence`
        (:`then_0`
          (`self.onFailed` (`self.DamagerPerFruit`)))))
    (:`then_1`
      (`/Engine/EditorBlueprintResources/StandardMacros.IsValid` Fruit
        (:`Is Valid`
          (`self.K2_DestroyActor` Fruit))))))

(event `StopTimer`
  ;[1 1 1] 타이머 정지
  (`|ExecutionSequence`
    (:`then_0`
      (`KismetSystemLibrary.PrintString` "Pawn called \"set Timer Stopped\""))
    (:`then_1`
      (bind _ashud (cast `/Game/UI/HUD` (`WidgetComponent.GetUserWidgetObject` (`self.HUDWidget`))))
      (`/Game/UI/HUD.setTimerStopped` _ashud))))

(event `SpawnFruitSixty`
  (bind _returnvalue (`KismetMathLibrary.Conv_IntToDouble` (`KismetMathLibrary.RandomIntegerInRange` -1000 1000)))
  (bind _x (.x (`SceneComponent.K2_GetComponentLocation` (`self.End`))))
  (bind _returnvalue_2 (`KismetMathLibrary.MakeVector` (- _x (`KismetMathLibrary.Sqrt` (- (`KismetMathLibrary.Square` (- (.x (`SceneComponent.K2_GetComponentLocation` (`self.Start`))) _x)) (`KismetMathLibrary.Square` (- (.y (`SceneComponent.K2_GetComponentLocation` (`self.End`))) _returnvalue))))) _returnvalue (`KismetMathLibrary.RandomFloatInRange` -110.0 -20.0)))
  ;[1 1 1] 60초 게임
  (`|ExecutionSequence`
    (:`then_0`
      (set `self.fruit_transform` (`KismetMathLibrary.MakeTransform` _returnvalue_2 (`KismetMathLibrary.FindLookAtRotation` _returnvalue_2 (`SceneComponent.K2_GetComponentLocation` (`self.End`)))))
      (set `self.fruit_type` (`KismetMathLibrary.RandomIntegerInRange` 0 4)))
    (:`then_1`
      (`self.Spawn Fruit Function`))
    (:`then_3`
      (bind _returnvalue_3 (`KismetSystemLibrary.K2_SetTimerDelegate` (delegate `SpawnFruitSixty`) (`KismetMathLibrary.RandomFloatInRange` 0.1 0.3)))
      (set `self.nextSpawnTimer` _returnvalue_3))))

(event `Spawn Fruit`
  (bind _returnvalue (`KismetMathLibrary.Conv_IntToDouble` (`KismetMathLibrary.RandomIntegerInRange` -1000 1000)))
  (bind _returnvalue_2 (* (`self.Difficulty`) 3.0))
  (bind _x (.x (`SceneComponent.K2_GetComponentLocation` (`self.End`))))
  (bind _returnvalue_3 (`KismetMathLibrary.MakeVector` (- _x (`KismetMathLibrary.Sqrt` (- (`KismetMathLibrary.Square` (- (.x (`SceneComponent.K2_GetComponentLocation` (`self.Start`))) _x)) (`KismetMathLibrary.Square` (- (.y (`SceneComponent.K2_GetComponentLocation` (`self.End`))) _returnvalue))))) _returnvalue (`KismetMathLibrary.RandomFloatInRange` -110.0 -20.0)))
  ;[1 1 1] 과일 생성
  (`|ExecutionSequence`
    (:`then_0`
      (set `self.fruit_transform` (`KismetMathLibrary.MakeTransform` _returnvalue_3 (`KismetMathLibrary.FindLookAtRotation` _returnvalue_3 (`SceneComponent.K2_GetComponentLocation` (`self.End`)))))
      (set `self.fruit_type` (`KismetMathLibrary.RandomIntegerInRange` 0 6)))
    (:`then_1`
      (`self.Spawn Fruit Function`)
      (if (< (`self.LoopCount`) 1)
        (set `self.LoopCount` (`KismetMathLibrary.RandomIntegerInRange` (`KismetMathLibrary.FTrunc` _returnvalue_2) (`KismetMathLibrary.FTrunc` (+ _returnvalue_2 3.0))))
        (`KismetSystemLibrary.PrintString` (`KismetStringLibrary.Conv_IntToString` (`self.LoopCount`)))
        (else
          (set `self.LoopCount` (- (`self.LoopCount`) 1)))))
    (:`then_2`
      (if (> (`self.LoopCount`) 0)
        (set `self.spawnRatio` 0.3)
        (else
          (set `self.spawnRatio` 5.0))))
    (:`then_3`
      (bind _returnvalue_4 (`KismetSystemLibrary.K2_SetTimerDelegate` (delegate `Spawn Fruit`) (`self.spawnRatio`)))
      (set `self.nextSpawnTimer` _returnvalue_4))))

(event `onFailed`
  (params (DamagePerFruit :type "Float (double-precision)"))
  ;[1 1 1] 과일 타격 실패시 점수 처리
  (`|ExecutionSequence`
    (:`then_0`
      (`KismetSystemLibrary.PrintString` "Update Health"))
    (:`then_1`
      (bind _output_get (set `self.Health` (`KismetMathLibrary.FClamp` (- (`self.Health`) DamagePerFruit) 0.0 100.0)))
      (bind _ashud (cast `/Game/UI/HUD` (`WidgetComponent.GetUserWidgetObject` (`self.HUDWidget`))))
      (set `/Game/UI/HUD.HealthPercentage` (/ _output_get 100.0) _ashud))
    (:`then_2`
      (if (<= (`self.Health`) 0.0)
        (bind _asbp_game_mode (cast `/Game/Blueprints/BP_GameMode` (`GameplayStatics.GetGameMode`)))
        (`/Game/Blueprints/BP_GameMode.StopGame` _asbp_game_mode)))))

(fn `Spawn Fruit Function`
  (`|SpawnActorFromClass` (select `int` (`self.fruit_type`) :`0` "/Game/Blueprints/BP_Fruits/BP_Apple.BP_Apple_C" :`1` "/Game/Blueprints/BP_Fruits/BP_Orange.BP_Orange_C" :`2` "/Game/Blueprints/BP_Fruits/BP_Apple.BP_Apple_C" :`3` "/Game/Blueprints/BP_Fruits/BP_Pear.BP_Pear_C" :`4` "/Game/Blueprints/BP_Fruits/BP_WaterMelon.BP_WaterMelon_C" :`5` "/Game/Blueprints/BP_Items/BP_Bomb.BP_Bomb_C" :`6` "/Game/Blueprints/BP_Items/BP_Itembox.BP_Itembox_C" :!type "Actor Class Reference") (`self.fruit_transform`) "Undefined" "MultiplyWithRoot" null null)
  (`AudioComponent.Play` (`self.Spawn_Sound`) 0.0))

(fn `UserConstructionScript`)