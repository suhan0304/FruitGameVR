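; BP_Blade is a VR test blade that cuts procedural meshes in two as it passes through them.
; Cube's begin overlap caches a procedural mesh through a DoOnce, which end overlap resets.
; End overlap also slices the cached mesh along the StaticMesh's location and up vector, capping the cut with M_Saber2.
; The new half then gets physics and a fixed impulse to fly off.
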(event `self.Cube.OnComponentBeginOverlap`
  (params (OverlappedComponent :type "PrimitiveComponent Object Reference") (OtherActor :type "Actor Object Reference") (OtherComp :type "PrimitiveComponent Object Reference") (OtherBodyIndex :type Integer) (bFromSweep :type Boolean) (SweepResult :type "HitResult Structure (by ref)"))
  (if true
    (`/Engine/EditorBlueprintResources/StandardMacros.DoOnce` false :!label _label
      (:`Completed`
        (bind `_as프로시저럴_메시_컴포넌트` (cast `ProceduralMeshComponent` OtherComp))))))

(event `self.Cube.OnComponentEndOverlap`
  (params (OverlappedComponent :type "PrimitiveComponent Object Reference") (OtherActor :type "Actor Object Reference") (OtherComp :type "PrimitiveComponent Object Reference") (OtherBodyIndex :type Integer))
  (bind _staticmesh (`self.StaticMesh`))
  (if true
    (`|ExecutionSequence`
      (:`then_0`
        (goto _label :!via `Reset`))
      (:`then_1`
        (`/Engine/EditorBlueprintResources/StandardMacros.IsValid` (stale `self.Cube.OnComponentBeginOverlap` `_as프로시저럴_메시_컴포넌트`)
          (:`Is Valid`
            _)
          (:`Is Not Valid`
            _))
        (bind _outotherhalfprocmesh (`KismetProceduralMeshLibrary.SliceProceduralMesh` (stale `self.Cube.OnComponentBeginOverlap` `_as프로시저럴_메시_컴포넌트`) (`SceneComponent.K2_GetComponentLocation` _staticmesh) (`SceneComponent.GetUpVector` _staticmesh) true "CreateNewSectionForCap" "/Game/Materials/M_Saber2.M_Saber2"))
        (`PrimitiveComponent.SetSimulatePhysics` _outotherhalfprocmesh true)
        (`PrimitiveComponent.AddImpulse` _outotherhalfprocmesh (300.0 300.0 300.0) "None" false)))))

(event `self.ReceiveTick`
  (params (DeltaSeconds :type "Float (single-precision)")))

(fn `UserConstructionScript`)