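; BP_Bomb is a hittable bomb actor in FruitArena that explodes once when hit.
; OnHit hides the collision and fruit meshes, plays the hit sound and destroys the actor a second later.
; When Chaos destruction is off, it also spawns an explosion particle and a BP_Chunks actor that inherits its materials and scales with the collision sphere radius.
; Its construction script only calls the parent's.
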(event `self.onHit`
  (`/Engine/EditorBlueprintResources/StandardMacros.DoOnce` false
    (:`Completed`
      (`|ExecutionSequence`
        (:`then_0`
          (`SceneComponent.SetVisibility` (`self.CollisionMesh`) false false)
          (`SceneComponent.SetVisibility` (`self.FruitMesh`) false false)
          (if (not (`self.shouldUseChaosDestruction`))
            (`|SpawnActorFromClass` "/Game/Blueprints/BP_Chunks.BP_Chunks_C" (`self.GetTransform`) "Undefined" "MultiplyWithRoot" null (`self.MainMaterial`) (`self.ChunkMaterial`) (/ (`SphereComponent.SphereRadius` (`self.CollisionMesh`)) 21.0) null)
            (`GameplayStatics.SpawnEmitterAtLocation` "/Game/Sample/StarterContent/Particles/P_Explosion.P_Explosion" (`self.K2_GetActorLocation`))))
        (:`then_1`
          (`KismetSystemLibrary.Delay` 1.0)
          (`self.K2_DestroyActor`))
        (:`then_2`
          (`AudioComponent.Play` (`self.HitSound`) 0.0))))))

(fn `UserConstructionScript`
  (`parent.UserConstructionScript`))