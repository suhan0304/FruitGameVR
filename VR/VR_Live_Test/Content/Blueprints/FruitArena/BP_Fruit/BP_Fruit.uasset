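; BP_Fruit is a launched, breakable fruit actor for FruitArena that bursts into chunks when hit.
; On BeginPlay it randomizes its container rotation and sets a random local forward velocity on its ProjectileMovement.
; The onHit event runs once, swapping the fruit for BP_Chunks scaled by collision radius, playing a sound and destroying the actor after a short delay.
; The construction script caches two FruitMesh materials to pass to the chunks.
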(event `self.ReceiveBeginPlay`
  (`SceneComponent.K2_SetWorldRotation` (`self.Container`) (`KismetMathLibrary.MakeRotator` (`KismetMathLibrary.RandomFloatInRange` -180.0 180.0) (`KismetMathLibrary.RandomFloatInRange` -180.0 180.0) (`KismetMathLibrary.RandomFloatInRange` -180.0 180.0)) false false)
  (`ProjectileMovementComponent.SetVelocityInLocalSpace` (`self.ProjectileMovement`) (`KismetMathLibrary.MakeVector` (`KismetMathLibrary.Conv_IntToDouble` (* (`KismetMathLibrary.RandomIntegerInRange` 1 5) 100)))))

(event `onHit`
  (`/Engine/EditorBlueprintResources/StandardMacros.DoOnce` false
    (:`Completed`
      (`|ExecutionSequence`
        (:`then_0`
          (`SceneComponent.SetVisibility` (`self.CollisionMesh`) false false)
          (`SceneComponent.SetVisibility` (`self.FruitMesh`) false false)
          (`|SpawnActorFromClass` "/Game/Blueprints/BP_Chunks.BP_Chunks_C" (`self.GetTransform`) "Undefined" "MultiplyWithRoot" null (`self.MainMaterial`) (`self.ChunkMaterial`) (/ (`SphereComponent.SphereRadius` (`self.CollisionMesh`)) 21.0) null)
          (`ActorComponent.K2_DestroyComponent` (`self.CollisionMesh`)))
        (:`then_1`
          (`KismetSystemLibrary.Delay` 1.0)
          (`self.K2_DestroyActor`))
        (:`then_2`
          (`AudioComponent.Play` (`self.HitSound`) 0.0))))))

(fn `UserConstructionScript`
  (bind _fruitmesh (`self.FruitMesh`))
  (set `self.MainMaterial` (`PrimitiveComponent.GetMaterial` _fruitmesh 0))
  (set `self.ChunkMaterial` (`PrimitiveComponent.GetMaterial` _fruitmesh 1)))