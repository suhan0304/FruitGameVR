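; BP_Hand is a VR motion-controller hand for a fruit-slicing game, configured as left or right, with sword setup on the right.
; While the sword is visible, overlaps score fruit with spawned score popups or trigger a random itembox effect: clearing all fruit or a print-only placeholder.
; Grabbing sphere-traces for a BP_GrabComponent, hiding the sword when one is found and otherwise toggling it.
; Grab and release also drive ABP_Hand's grasp pose.
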(event `self.ReceiveBeginPlay`
  (bind _handmesh (`self.HandMesh`))
  (bind _handmesh_2 (`self.HandMesh`))
  (bind _bp_sword (`self.BP_Sword`))
  (`|ExecutionSequence`
    (:`then_0`
      (if (`self.bLeftHand`)
        (`SkeletalMeshComponent.SetSkeletalMeshAsset` (`self.HandMesh`) "/Game/Sample/Characters/MannequinsXR/Meshes/SKM_MannyXR_left.SKM_MannyXR_left")
        (`SceneComponent.K2_SetRelativeRotation` _handmesh_2 (struct :`Pitch` -90.0 :`Roll` -90.0) false false)
        (`PrimitiveComponent.SetMaterial` _handmesh_2 0 "/Game/Materials/M_Hand.M_Hand")
        (set `MotionControllerComponent.MotionSource` "Left" (`self.MotionController`))
        (`ActorComponent.K2_DestroyComponent` (`self.Sword`))
        (else
          (`|ExecutionSequence`
            (:`then_0`
              (`SkeletalMeshComponent.SetSkeletalMeshAsset` (`self.HandMesh`) "/Game/Sample/Characters/MannequinsXR/Meshes/SKM_MannyXR_right.SKM_MannyXR_right")
              (`SceneComponent.K2_SetRelativeRotation` _handmesh (struct :`Pitch` 90.0 :`Roll` 90.0) false false)
              (`PrimitiveComponent.SetMaterial` _handmesh 0 "/Game/Materials/M_Hand.M_Hand")
              (set `MotionControllerComponent.MotionSource` "Right" (`self.MotionController`)))
            (:`then_1`
              (`SceneComponent.SetVisibility` _bp_sword true false)
              (`ActorComponent.Activate` _bp_sword false)
              (`/Engine/EditorBlueprintResources/StandardMacros.DoOnce` false
                (:`Completed`
                  (`SceneComponent.K2_AddRelativeRotation` _bp_sword (struct :`Yaw` 200.0) false false)
                  (`SceneComponent.K2_AddRelativeLocation` _bp_sword (-24.0 0.0 0.0) false true))))))))
    (:`then_1`
      (set `self.InitHandMeshRelativeTransform` (`SceneComponent.GetRelativeTransform` (`self.HandMesh`))))))

(event `self.Sword.OnComponentBeginOverlap`
  (params (OverlappedComponent :type "PrimitiveComponent Object Reference") (OtherActor :type "Actor Object Reference") (OtherComp :type "PrimitiveComponent Object Reference") (OtherBodyIndex :type Integer) (bFromSweep :type Boolean) (SweepResult :type "HitResult Structure (by ref)"))
  (if (`SceneComponent.IsVisible` (`self.BP_Sword`))
    (bind _asbp_fruit (cast `/Game/Blueprints/FruitArena/BP_Fruit/BP_Fruit` OtherActor))
    (if (!= (`GameplayStatics.GetObjectClass` _asbp_fruit) "/Game/Blueprints/FruitArena/BP_Itembox.BP_Itembox_C")
      (`self.onFruitHit` _asbp_fruit)
      (else
        (`self.onItemboxHit` _asbp_fruit)))))

(event `onFruitHit`
  (params (Fruit :type "/Game/Blueprints/FruitArena/BP_Fruit/BP_Fruit Object Reference"))
  (bind _score (`/Game/Blueprints/FruitArena/BP_Fruit/BP_Fruit.Score` Fruit))
  (if (`SceneComponent.IsVisible` (`/Game/Blueprints/FruitArena/BP_Fruit/BP_Fruit.FruitMesh` Fruit))
    (`/Game/Blueprints/FruitArena/BP_Fruit/BP_Fruit.onHit` Fruit)
    (`|SpawnActorFromClass` "/Game/Blueprints/FruitArena/BP_Score.BP_Score_C" (`KismetMathLibrary.MakeTransform` (`self.K2_GetActorLocation` Fruit) (struct :`Yaw` 180.0)) "Undefined" "MultiplyWithRoot" null _score null)
    (bind _asbp_game_mode (cast `/Game/Blueprints/BP_GameMode` (`GameplayStatics.GetGameMode`)))
    (`/Game/Blueprints/BP_GameMode.addScore` _asbp_game_mode _score)))

(event `onItemboxHit`
  (params (Fruit :type "/Game/Blueprints/FruitArena/BP_Fruit/BP_Fruit Object Reference"))
  ;[1 1 1] 아이템 히트시
  (`self.K2_DestroyActor` Fruit)
  (switch `int` (`KismetMathLibrary.RandomIntegerInRange` 0 1)
    (:`0`
      (`KismetSystemLibrary.PrintString` "Item 0 적용")
      (bind _outactors (`GameplayStatics.GetAllActorsOfClass` "/Game/Blueprints/FruitArena/BP_Fruit/BP_Fruit.BP_Fruit_C"))
      (for _array_element _outactors
        (bind _returnvalue (`GameplayStatics.GetObjectClass` _array_element))
        (if (or (!= _returnvalue "/Game/Blueprints/FruitArena/BP_Bomb.BP_Bomb_C") (!= _returnvalue null))
          (`self.onFruitHit` _array_element)
          (else
            (`self.K2_DestroyActor` _array_element)))))
    (:`1`
      (`KismetSystemLibrary.PrintString` "Item 1 적용"))))

(fn `FindGrabComponentNearHand`
  (returns (HeldTarget :type "/Game/Blueprints/BP_GrabComponent Object Reference"))
  (locals (LocalGrapPosition :type "Vector Structure" :default (0.0 0.0 0.0)) (LocalGrapComponent :type "/Game/Blueprints/BP_GrabComponent Object Reference"))
  (`|ExecutionSequence`
    (:`then_0`
      (bind _output_get (set `local.LocalGrapPosition` (`SceneComponent.K2_GetComponentLocation` (`self.MotionController`))))
      (bind (_outhit _returnvalue) (`KismetSystemLibrary.SphereTraceSingleForObjects` :`Start` _output_get :`End` _output_get :`Radius` (`self.GrapRadius`) :`ObjectTypes` (`|MakeArray` "ObjectTypeQuery7" :!type "EObjectTypeQuery Enum") :`DrawDebugType` "ForDuration" :`DrawTime` 1.0))
      (if _returnvalue
        (bind _returnvalue_2 (`self.GetComponentByClass` (`.HitActor` (`GameplayStatics.BreakHitResult` _outhit)) "/Game/Blueprints/BP_GrabComponent.BP_GrabComponent_C"))
        (`/Engine/EditorBlueprintResources/StandardMacros.IsValid` _returnvalue_2
          (:`Is Valid`
            (set `local.LocalGrapComponent` _returnvalue_2)))))
    (:`then_1`
      (return (`local.LocalGrapComponent`)))))

(fn `HandleGrab`
  (bind _bp_sword (`self.BP_Sword`))
  (`|ExecutionSequence`
    (:`then_0`
      (bind _heldtarget (`self.FindGrabComponentNearHand`))
      (`/Engine/EditorBlueprintResources/StandardMacros.IsValid` _heldtarget
        (:`Is Valid`
          (`|ExecutionSequence`
            (:`then_0`
              (bind _bsuccess (`/Game/Blueprints/BP_GrabComponent.TryGrab` _heldtarget self))
              (if _bsuccess
                (bind _output_get (set `self.HeldComponent` _heldtarget))
                (`/Game/Blueprints/BP_GrabComponent.OnGrabbed` _output_get)))
            (:`then_1`
              (`SceneComponent.SetVisibility` _bp_sword false false :!label _label))))
        (:`Is Not Valid`
          (if (`SceneComponent.IsVisible` _bp_sword)
            (goto _label)
            (else
              (`SceneComponent.SetVisibility` _bp_sword true false))))))
    (:`then_1`
      (bind _asabp_hand (cast `/Game/Resources/Hand/ABP_Hand` (`SkeletalMeshComponent.GetAnimInstance` (`self.HandMesh`))))
      (set `/Game/Resources/Hand/ABP_Hand.PoseAlphaGrasp` 1.0 _asabp_hand))))

(fn `HandleRelease`
  (bind _heldcomponent (`self.HeldComponent`))
  (`|ExecutionSequence`
    (:`then_0`
      (`/Engine/EditorBlueprintResources/StandardMacros.IsValid` _heldcomponent
        (:`Is Valid`
          (`/Game/Blueprints/BP_GrabComponent.TryRelease` _heldcomponent)
          (`/Game/Blueprints/BP_GrabComponent.OnDropped` _heldcomponent))))
    (:`then_1`
      (bind _asabp_hand (cast `/Game/Resources/Hand/ABP_Hand` (`SkeletalMeshComponent.GetAnimInstance` (`self.HandMesh`))))
      (set `/Game/Resources/Hand/ABP_Hand.PoseAlphaGrasp` 0.0 _asabp_hand))))

(fn `ResetHandMesh`
  (`SceneComponent.K2_AttachToComponent` (`self.HandMesh`) (`self.MotionController`) "None" "KeepWorld" "KeepWorld" "KeepWorld" true)
  (`SceneComponent.K2_SetRelativeTransform` (`self.HandMesh`) (`self.InitHandMeshRelativeTransform`) false true))

(fn `UserConstructionScript`)