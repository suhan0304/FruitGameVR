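; BP_Gun is a grabbable VR gun that fires projectiles from its muzzle.
; Grabbing it through BP_GrabComponent enables input on the actor and adds the left or right weapon mapping context for the grabbing hand, while dropping it reverses both.
; Separate left and right Enhanced Input shoot actions check the grabbing hand, then share one spawn of the Projectile class at MuzzleLocation, with the player pawn as instigator.
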(event `self.BP_GrabComponent.OnGrabbed`
  (`self.EnableInput` (`GameplayStatics.GetPlayerController` 0))
  (`EnhancedInputSubsystemInterface.AddMappingContext` (pcsubsystem `EnhancedInputLocalPlayerSubsystem` (`GameplayStatics.GetPlayerController` 0)) (select `bool` (`|EnumEquality` (`/Game/Blueprints/BP_GrabComponent.GetGrabbingHandType` (`self.BP_GrabComponent`)) "Left") :`false` "/Game/Blueprints/Input/IMC_VR_Weapon_Right.IMC_VR_Weapon_Right" :`true` "/Game/Blueprints/Input/IMC_VR_Weapon_Left.IMC_VR_Weapon_Left" :!type "InputMappingContext Object Reference") 0 (struct))
  (`KismetSystemLibrary.PrintString` "Hello"))

(event `self.BP_GrabComponent.OnDropped`
  (`self.DisableInput` (`GameplayStatics.GetPlayerController` 0))
  (`EnhancedInputSubsystemInterface.RemoveMappingContext` (pcsubsystem `EnhancedInputLocalPlayerSubsystem` (`GameplayStatics.GetPlayerController` 0)) (select `bool` (`|EnumEquality` (`/Game/Blueprints/BP_GrabComponent.GetGrabbingHandType` (`self.BP_GrabComponent`)) "Left") :`false` "/Game/Blueprints/Input/IMC_VR_Weapon_Right.IMC_VR_Weapon_Right" :`true` "/Game/Blueprints/Input/IMC_VR_Weapon_Left.IMC_VR_Weapon_Left" :!type "InputMappingContext Object Reference") (struct)))

(event `EnhancedInput|/Game/Blueprints/Input/Actions/IA_VR_Shoot_Left`
  (params (ActionValue :type "Float (double-precision)") (ElapsedSeconds :type "Float (double-precision)") (TriggeredSeconds :type "Float (double-precision)") (InputAction :type "InputAction Object Reference" :default "/Game/Blueprints/Input/Actions/IA_VR_Shoot_Left.IA_VR_Shoot_Left"))
  (bind _muzzlelocation (`self.MuzzleLocation`))
  (:`Started`
    (if (`|EnumEquality` (`/Game/Blueprints/BP_GrabComponent.GetGrabbingHandType` (`self.BP_GrabComponent`)) "Left")
      (`|SpawnActorFromClass` "/Game/Sample/VRTemplate/Blueprints/Projectile.Projectile_C" (`KismetMathLibrary.MakeTransform` (`SceneComponent.K2_GetComponentLocation` _muzzlelocation) (`SceneComponent.K2_GetComponentRotation` _muzzlelocation)) "AlwaysSpawn" "MultiplyWithRoot" self (`GameplayStatics.GetPlayerPawn` 0) :!label _label))))

(event `EnhancedInput|/Game/Blueprints/Input/Actions/IA_VR_Shoot_Right`
  (params (ActionValue :type "Float (double-precision)") (ElapsedSeconds :type "Float (double-precision)") (TriggeredSeconds :type "Float (double-precision)") (InputAction :type "InputAction Object Reference" :default "/Game/Blueprints/Input/Actions/IA_VR_Shoot_Right.IA_VR_Shoot_Right"))
  (:`Started`
    (if (`|EnumEquality` (`/Game/Blueprints/BP_GrabComponent.GetGrabbingHandType` (`self.BP_GrabComponent`)) "Right")
      (goto _label))))

(fn `UserConstructionScript`)