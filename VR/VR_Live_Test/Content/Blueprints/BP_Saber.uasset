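; BP_Saber is a blade actor that cuts procedural meshes it passes through.
; On blade begin overlap, it changes the touched component's material and caches it as a procedural mesh through a DoOnce.
; On end overlap, it resets the DoOnce and slices the cached mesh along a plane from the Point component's location and up vector, adding a glowing cap.
; The new half then simulates physics and receives a fixed impulse.
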(event `self.Blade.OnComponentBeginOverlap`
  (params (OverlappedComponent :type "PrimitiveComponent Object Reference") (OtherActor :type "Actor Object Reference") (OtherComp :type "PrimitiveComponent Object Reference") (OtherBodyIndex :type Integer) (bFromSweep :type Boolean) (SweepResult :type "HitResult Structure (by ref)"))
  (if true
    (`|ExecutionSequence`
      (:`then_0`
        (`PrimitiveComponent.SetMaterial` OtherComp 0 "/Engine/MapTemplates/Materials/BasicAsset01.BasicAsset01"))
      (:`then_1`
        (`/Engine/EditorBlueprintResources/StandardMacros.DoOnce` false :!label _label
          (:`Completed`
            (bind _asprocedural_mesh_component (cast `ProceduralMeshComponent` OtherComp))))))))

(event `self.Blade.OnComponentEndOverlap`
  (params (OverlappedComponent :type "PrimitiveComponent Object Reference") (OtherActor :type "Actor Object Reference") (OtherComp :type "PrimitiveComponent Object Reference") (OtherBodyIndex :type Integer))
  (bind _point (`self.Point`))
  (if true
    (`|ExecutionSequence`
      (:`then_0`
        (goto _label :!via `Reset`))
      (:`then_1`
        (`/Engine/EditorBlueprintResources/StandardMacros.IsValid` (stale `self.Blade.OnComponentBeginOverlap` _asprocedural_mesh_component)
          (:`Is Valid`
            _)
          (:`Is Not Valid`
            _))
        (bind _outotherhalfprocmesh (`KismetProceduralMeshLibrary.SliceProceduralMesh` (stale `self.Blade.OnComponentBeginOverlap` _asprocedural_mesh_component) (`SceneComponent.K2_GetComponentLocation` _point) (`SceneComponent.GetUpVector` _point) true "CreateNewSectionForCap" "/Game/Blueprints/Materials/M_Glow.M_Glow"))
        (`PrimitiveComponent.SetSimulatePhysics` _outotherhalfprocmesh true)
        (`PrimitiveComponent.AddImpulse` _outotherhalfprocmesh (300.0 300.0 300.0) "None" true)))))

(fn `UserConstructionScript`)