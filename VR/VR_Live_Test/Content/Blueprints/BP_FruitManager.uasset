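; BP_FruitManager is the spawner actor for a fruit game, launching random fruits, bombs or item boxes from randomized points around SpawnZone, aimed at End.
; BeginPlay starts spawning after delays; SpawnFruit then reschedules itself on a random timer scaled by SpawnRatio.
; A Box overlap silently destroys bombs, while missed fruits damage BP_Pawn through OnFailed before being destroyed.
; StopGame clears the spawn timer and removes all BP_Fruit actors.
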(event `self.ReceiveBeginPlay`
  (`|ExecutionSequence`
    (:`then_0`
      (`KismetSystemLibrary.ExecuteConsoleCommand` "stat fps" null))
    (:`then_1`
      (`KismetSystemLibrary.Delay` 2.0)
      (`self.StartGame`))))

(event `StartGame`
  (`KismetSystemLibrary.Delay` 3.0)
  (`self.Spawn Fruit`))

(event `StopGame`
  (`|ExecutionSequence`
    (:`then_0`
      (`KismetSystemLibrary.K2_ClearAndInvalidateTimerHandle` (`self.nextSpawnTimer`)))
    (:`then_1`
      (`self.removeAllFruits`))))

(event `Spawn Fruit`
  (bind _spawnzone (`self.SpawnZone`))
  (bind _sphereradius (`SphereComponent.SphereRadius` _spawnzone))
  (bind _returnvalue (+ (`SceneComponent.K2_GetComponentLocation` _spawnzone) (* (* _sphereradius (0.0 0.0 1.0)) (`KismetMathLibrary.RandomIntegerInRange` -3 3)) (* (* _sphereradius (0.0 10.0 0.0)) (`KismetMathLibrary.RandomIntegerInRange` -2 2))))
  (`|ExecutionSequence`
    (:`then_0`
      (`|SpawnActorFromClass` (select `int` (`KismetMathLibrary.RandomIntegerInRange` 0 6) :`0` "/Game/Blueprints/FruitArena/BP_Apple.BP_Apple_C" :`1` "/Game/Blueprints/FruitArena/BP_Orange.BP_Orange_C" :`2` "/Game/Blueprints/FruitArena/BP_Mango.BP_Mango_C" :`3` "/Game/Blueprints/FruitArena/BP_Pear.BP_Pear_C" :`4` "/Game/Blueprints/FruitArena/BP_WaterMelon.BP_WaterMelon_C" :`5` "/Game/Blueprints/FruitArena/BP_Bomb.BP_Bomb_C" :`6` "/Game/Blueprints/FruitArena/BP_Itembox.BP_Itembox_C" :!type "Actor Class Reference") (`KismetMathLibrary.MakeTransform` _returnvalue (`KismetMathLibrary.FindLookAtRotation` _returnvalue (`KismetMathLibrary.RandomPointInBoundingBox` (`SceneComponent.K2_GetComponentLocation` (`self.End`)) (1.0 1.0 1.0)))) "Undefined" "MultiplyWithRoot" null null))
    (:`then_1`
      (bind _returnvalue_2 (`KismetSystemLibrary.K2_SetTimerDelegate` (delegate `Spawn Fruit`) (/ (`KismetMathLibrary.RandomFloatInRange` 3.0 7.0) (`KismetMathLibrary.FMax` (`self.spawnRatio`) 0.25))))
      (set `self.nextSpawnTimer` _returnvalue_2))))

(event `self.Box.OnComponentBeginOverlap`
  (params (OverlappedComponent :type "PrimitiveComponent Object Reference") (OtherActor :type "Actor Object Reference") (OtherComp :type "PrimitiveComponent Object Reference") (OtherBodyIndex :type Integer) (bFromSweep :type Boolean) (SweepResult :type "HitResult Structure (by ref)"))
  (if (== "/Game/Blueprints/FruitArena/BP_Bomb.BP_Bomb_C" (`GameplayStatics.GetObjectClass` OtherActor))
    (`self.K2_DestroyActor` OtherActor)
    (else
      (bind _asbp_fruit (cast `/Game/Blueprints/FruitArena/BP_Fruit/BP_Fruit` OtherActor))
      (`self.fruitFailed` _asbp_fruit))))

(event `fruitFailed`
  (params (Fruit :type "/Game/Blueprints/FruitArena/BP_Fruit/BP_Fruit Object Reference"))
  (`|ExecutionSequence`
    (:`then_0`
      (cast `/Game/Blueprints/BP_GameMode` (`GameplayStatics.GetGameMode`))
      (`|ExecutionSequence`
        (:`then_1`
          (bind _returnvalue (`GameplayStatics.GetActorOfClass` "/Game/Blueprints/BP_Pawn.BP_Pawn_C"))
          (`/Game/Blueprints/BP_Pawn.onFailed` _returnvalue (`self.DamagerPerFruit`)))))
    (:`then_1`
      (`/Engine/EditorBlueprintResources/StandardMacros.IsValid` Fruit
        (:`Is Valid`
          (`self.K2_DestroyActor` Fruit))))))

(event `removeAllFruits`
  (bind _outactors (`GameplayStatics.GetAllActorsOfClass` "/Game/Blueprints/FruitArena/BP_Fruit/BP_Fruit.BP_Fruit_C"))
  (for _array_element _outactors
    (`self.K2_DestroyActor` _array_element)))

(fn `UserConstructionScript`)