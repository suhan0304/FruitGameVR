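; BP_Cube is a moving cube actor that travels along its local negative X axis and removes itself once out of bounds.
; The construction script copies the Cube static mesh into a ProceduralMesh component with collision.
; Tick offsets that procedural mesh by a fixed step without sweeping, so speed depends on frame rate.
; The actor destroys itself when the mesh passes a world X limit or drops to a low Z height.
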(event `self.ReceiveTick`
  (params (DeltaSeconds :type "Float (single-precision)"))
  (bind (_returnvalue_x _returnvalue_y _returnvalue_z) (`KismetMathLibrary.BreakVector` (`SceneComponent.K2_GetComponentLocation` (`self.ProceduralMesh`))))
  (`SceneComponent.K2_AddLocalOffset` (`self.ProceduralMesh`) (-20.0 0.0 0.0) false false)
  (if (or (<= _returnvalue_x -2000.0) (<= _returnvalue_z 30.0))
    (`self.K2_DestroyActor`)))

(fn `UserConstructionScript`
  (`KismetProceduralMeshLibrary.CopyProceduralMeshFromStaticMeshComponent` (`self.Cube`) 0 (`self.ProceduralMesh`) true))